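; BP_Tower is a tower actor that tracks BP_Enemy actors and fires bullets at them.
; Overlaps on its Radius component maintain EnemyArray, with debug prints on entry and exit.
; Attack spawns a BP_Bullet at ArmPos and passes it the target, using a DoOnce reset after AttackSpeed seconds as cooldown.
; RotateToEnemy yaws the Cube toward its target in an endless short-delay loop; neither event is called within this graph.
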(event OnComponentBeginOverlap(Radius)
  (params (OverlappedComponent :type Primitive%20Component%20Object%20Reference) (OtherActor :type Actor%20Object%20Reference) (OtherComp :type Primitive%20Component%20Object%20Reference) (OtherBodyIndex :type Integer) (bFromSweep :type Boolean) (SweepResult :type Hit%20Result%20Structure%20%28by%20ref%29))
  ;[1 1 1] GetEnemys
  (bind _asbp_enemy (Utilities|Casting|CastToBP_Enemy OtherActor))
  (Utilities|Array|Add (Variables|Default|GetEnemyArray) _asbp_enemy)
  (Development|PrintString (Utilities|String|Append (Utilities|GetDisplayName self) "get Enemy")))

(event OnComponentEndOverlap(Radius)
  (params (OverlappedComponent :type Primitive%20Component%20Object%20Reference) (OtherActor :type Actor%20Object%20Reference) (OtherComp :type Primitive%20Component%20Object%20Reference) (OtherBodyIndex :type Integer))
  ;[1 1 1] GetEnemys
  (bind _asbp_enemy (Utilities|Casting|CastToBP_Enemy OtherActor))
  (Utilities|Array|RemoveItem (Variables|Default|GetEnemyArray) _asbp_enemy)
  (Development|PrintString (Utilities|String|Append (Utilities|GetDisplayName self) "Remove Enemy")))

(event Custom|Attack
  (params (Enemy :type Actor%20Object%20Reference))
  ;[1 1 1] Attack
  (Utilities|IsValid Enemy
    (:Is%20Valid
      (Utilities|FlowControl|DoOnce false :!label _label
        (:Completed
          (bind _returnvalue (Game|SpawnActorfromClass "/Game/BluePrints/Tower/BP_Bullet.BP_Bullet_C" (Math|Transform|MakeTransform (Transformation|GetWorldLocation (Variables|Default|GetArmPos))) "AdjustIfPossibleButDontSpawnIfColliding" 0 0))
          (Default|AttacktoEnemy _returnvalue Enemy)
          (Utilities|FlowControl|Delay (Variables|Default|GetAttackSpeed))
          (goto _label Reset))))))

(event Custom|RotateToEnemy
  (params (Enemy :type Actor%20Object%20Reference))
  (bind _cube (Variables|Default|GetCube))
  ;[1 1 1] RotateToEnemy
  (Transformation|SetWorldRotation _cube (Math|Rotator|MakeRotator 0.0 0.0 (.yaw (Math|Rotator|FindLookatRotation (Transformation|GetWorldLocation _cube) (Transformation|GetActorLocation Enemy)))) false false :!label _label)
  (Utilities|FlowControl|Delay 0.01)
  (goto _label))

(fn ConstructionScript)