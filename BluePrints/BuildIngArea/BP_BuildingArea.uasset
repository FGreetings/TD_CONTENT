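; BP_BuildingArea is a build slot where towers are placed.
; BuildTower spawns the given tower class at the ChoosenArea component's location with zero rotation, always spawning regardless of collision, then marks the slot as full.
; BeingSelected and NotBeingSelected show selection state by swapping the frame material on its four mesh components.
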(event Custom|BuildTower
  (params (ShouldBuildTower :type Actor%20Class%20Reference))
  ;[1 1 1] 建造
  (Game|SpawnActorfromClass ShouldBuildTower (Math|Transform|MakeTransform (Transformation|GetWorldLocation (Variables|Default|GetChoosenArea))) "AlwaysSpawn" 0 0)
  (Variables|Default|SetIsFull true))

(event Custom|NotBeingSelected
  ;[1 1 1] 未被选中
  (Rendering|Material|SetMaterial (Variables|Default|GetStaticMesh) 0 "/Game/BluePrints/BuildIngArea/M_BuildAreaShowingFrame.M_BuildAreaShowingFrame"))

(event Custom|BeingSelected
  ;[1 1 1] 被选择
  (Rendering|Material|SetMaterial (Variables|Default|GetStaticMesh) 0 "/Game/BluePrints/BuildIngArea/M_BuildAreaShowingFrame_BeingChoosen.M_BuildAreaShowingFrame_BeingChoosen"))

(event EventBeginPlay)

(event Collision|EventActorBeginOverlap
  (params (OtherActor :type Actor%20Object%20Reference)))

(event EventTick
  (params (DeltaSeconds :type Float%20%28single-precision%29)))

(fn ConstructionScript)