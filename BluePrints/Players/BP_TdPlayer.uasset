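; Player pawn for what appears to be a tower-defense game, providing a top-down camera and building-area selection.
; Each tick, helper functions pan the actor along its own axes, apparently when the cursor nears a viewport edge.
; An input axis yaws the actor, and the mouse wheel adjusts spring-arm length.
; Left-click traces under the cursor to select a BP_BuildingArea, locking selection and flagging the widget if not full; right-click deselects.
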(event Custom|RemoveSelectedBuildingArea
  ;[1 1 1] 取消选中当前BuildingArea
  (Default|NotBeingSelected (Utilities|Array|Get(acopy) (Variables|Default|GetSelectedAreas)))
  (Variables|Default|SetIsChoosenArea false)
  (Variables|Default|SetShouldWidgetShow false)
  (Utilities|Array|RemoveIndex (Variables|Default|GetSelectedAreas)))

(event EventTick
  (params (DeltaSeconds :type Float%20%28single-precision%29))
  (bind (_isright _isleft) (|判断相机是否该左右移动))
  (bind (_isup _isdown) (|判断是否该上下移动))
  ;[1 1 1] CameraMovement
  (Utilities|FlowControl|Sequence
    (:then_0
      (|相机上下移动 _isup _isdown))
    (:then_1
      (|相机左右移动 _isright _isleft))))

(event Input|AxisEvents|InputAxisCameraRotateToLeft
  (params (AxisValue :type Float%20%28single-precision%29))
  ;[1 1 1] CameraRotate
  (Class|Actor|AddActorWorldRotation (Math|Rotator|MakeRotator 0.0 0.0 (* AxisValue 3.0))))

(event Input|MouseEvents|MouseWheelUp
  (params (Key :type Key%20Structure :default "AnyKey"))
  (bind _springarm (Variables|Default|GetSpringArm))
  ;[1 1 1] Camera +/-
  (:Pressed
    (if (> (Variables|/Script/Engine.SpringArmComponent|GetTargetArmLength _springarm) -5e+02)
      (Variables|/Script/Engine.SpringArmComponent|SetTargetArmLength _springarm (- (Variables|/Script/Engine.SpringArmComponent|GetTargetArmLength _springarm) (Variables|Default|GetCameraSpeed))))))

(event Input|MouseEvents|LeftMouseButton
  (params (Key :type Key%20Structure :default "AnyKey"))
  ;[1 1 1] GetBuildingArea
  (:Pressed
    (if (not (Variables|Default|GetIsChoosenArea))
      (bind _asbp_building_area (Utilities|Casting|CastToBP_BuildingArea (.HitActor (Collision|BreakHitResult (.HitResult (Game|Player|GetHitResultUnderCursorbyChannel (Game|GetPlayerController 0) "TraceTypeQuery1" true))))))
      (bind _output_get (Variables|Default|SetSelectedAreas (Utilities|Array|MakeArray _asbp_building_area)))
      (Default|BeingSelected (Utilities|Array|Get(acopy) _output_get))
      (if (not (Variables|/Game/BluePrints/BuildIngArea/BP_BuildingArea.BP_BuildingArea_C|GetIsFull (Utilities|Array|Get(acopy) _output_get)))
        (Variables|Default|SetIsChoosenArea true)
        (Variables|Default|SetShouldWidgetShow true)))))

(event Input|MouseEvents|MouseWheelDown
  (params (Key :type Key%20Structure :default "AnyKey"))
  (bind _springarm (Variables|Default|GetSpringArm))
  ;[1 1 1] Camera +/-
  (:Pressed
    (if (< (Variables|/Script/Engine.SpringArmComponent|GetTargetArmLength _springarm) 1e+03)
      (Variables|/Script/Engine.SpringArmComponent|SetTargetArmLength _springarm (+ (Variables|/Script/Engine.SpringArmComponent|GetTargetArmLength _springarm) (Variables|Default|GetCameraSpeed))))))

(event Input|MouseEvents|RightMouseButton
  (params (Key :type Key%20Structure :default "AnyKey"))
  ;[1 1 1] 鼠标右键点击后取消选中
  (:Pressed
    (CallFunction|RemoveSelectedBuildingArea)))

(fn ConstructionScript)