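; BP_Enemy is an enemy Blueprint with health and movement speed that dies when its HP runs out.
; On BeginPlay it applies its Speed variable to the character movement's max walk speed and prints the value.
; AnyDamage subtracts damage from HP, calls CalculateHealth to destroy the actor at zero or below, and prints the remaining HP for debugging.
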(event Custom|CalculateHealth
  (if (<= (Variables|Default|GetHP) 0.0)
    (Actor|DestroyActor)))

(event EventBeginPlay
  (bind _output_get (Variables|/Script/Engine.CharacterMovementComponent|SetMaxWalkSpeed (Variables|Character|GetCharacterMovement) (Variables|Default|GetSpeed)))
  (Development|PrintString (Utilities|String|ToString(Float) _output_get)))

(event Collision|EventActorBeginOverlap
  (params (OtherActor :type Actor%20Object%20Reference)))

(event EventTick
  (params (DeltaSeconds :type Float%20%28single-precision%29)))

(event Game|Damage|EventAnyDamage
  (params (Damage :type Float%20%28single-precision%29) (DamageType :type Damage%20Type%20Object%20Reference) (InstigatedBy :type Controller%20Object%20Reference) (DamageCauser :type Actor%20Object%20Reference))
  ;[1 1 1] GetDamage
  (Variables|Default|SetHP (- (Variables|Default|GetHP) Damage))
  (CallFunction|CalculateHealth)
  (Development|PrintString (Utilities|String|Append (Utilities|GetDisplayName self) "    HP:     " (Utilities|String|ToString(Float) (Variables|Default|GetHP)))))

(fn ConstructionScript)